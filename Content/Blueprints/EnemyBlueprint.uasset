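; Enemy actor for a shooter that slides sideways, fires bullets and dies when hit by the player's shots.
; Each tick it moves along Y at a fixed speed, taking its direction from DirectionY on MyGameState.
; A countdown timer in ShotBullet spawns an enemy bullet just below it at random intervals.
; Overlap with a player bullet spawns an explosion, sends score to the GameState and destroys the enemy.
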(event Collision|EventActorBeginOverlap
  (params (OtherActor :type Actor%20Object%20Reference))
  ;[1 1 1] 弾があたった時
  (Utilities|Casting|CastToPlayerBulletBlueprint OtherActor) ; プレイヤーが放った弾の場合のみ
  (Game|SpawnActorfromClass "/Game/StarterContent/Blueprints/Blueprint_Effect_Explosion.Blueprint_Effect_Explosion_C" (Math|Conversions|ToTransform(Vector) (Transformation|GetActorLocation)) "Undefined" 0 0)
  (Class|MyInterface|AddScore(Message) (Game|GetGameState) 10)
  (Actor|DestroyActor))

(event EventTick
  (params (DeltaSeconds :type Float%20%28single-precision%29))
  ;[1 1 1] 移動
  (Transformation|SetActorLocation (+ (* (* "0,1.000000,0.000000" (Variables|/Game/Blueprints/MyGameState.MyGameState_C|GetDirectionY (.AsMy%20Game%20State (Utilities|Casting|CastToMyGameState (Game|GetGameState))))) (* "0,50.000000,0.000000" DeltaSeconds)) (Transformation|GetActorLocation)) false false)
  (CallFunction|ShotBullet DeltaSeconds))

(fn ConstructionScript)

(fn ShotBullet
  (params (DeltaTime :type Float%20%28single-precision%29))
  (if (< (- (Variables|Default|GetShotTimer) DeltaTime) 0.0)
    (Game|SpawnActorfromClass "/Game/Blueprints/EnemyBulletBlueprint.EnemyBulletBlueprint_C" (Math|Conversions|ToTransform(Vector) (+ (Transformation|GetActorLocation) "0, 0,-60.000000")) "Undefined" 0 0)
    (Variables|Default|SetShotTimer (Math|Random|RandomFloatinRange 1.0 2.0))
    (else
      (Variables|Default|SetShotTimer (- (Variables|Default|GetShotTimer) DeltaTime)))))