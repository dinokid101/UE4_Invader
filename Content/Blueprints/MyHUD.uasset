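; HUD Blueprint that draws the score text and player health bar on the canvas each frame, scaled relative to a 640-pixel screen width.
; DrawHUD reads score from the GameState, then calls DrawHealthBar, which reads health from player pawn 0.
; The bar crops the lower half of the Health texture by health percentage, then overlays the upper half at full width.
; GetHealth and GetScore are unused here and return zero.
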(event EventDrawHUD
  (params (SizeX :type Integer) (SizeY :type Integer))
  (bind _returnvalue (Math|Conversions|ToFloat(Integer) SizeX))
  (bind _returnvalue_2 (/ _returnvalue 6.4e+02))
  ;[1 1 1] スコア表示
  (bind _score (Class|MyInterface|GetScore(Message) (Game|GetGameState)))
  (HUD|DrawText (Utilities|String|BuildString(Integer) "" "Score:" _score) "(R=1.000000,G=1.000000,B=1.000000,A=1.000000)" 2e+01 1e+01 "/Engine/EngineFonts/RobotoDistanceField.RobotoDistanceField" _returnvalue_2 true)
  (CallFunction|DrawHealthBar "(X=490.000000,Y=15.000000)" _returnvalue_2))

(fn ConstructionScript)

(fn DrawHealthBar
  (params (InPosition :type Vector%202D%20Structure) (InScale :type Float%20%28single-precision%29))
  (bind (_x _y) (Math|Vector2D|BreakVector2D InPosition))
  (bind _health (Class|MyInterface|GetHealth(Message) (Game|Player|GetPlayerPawn 0)))
  (Canvas|DrawTexture "/Game/Textures/Health.Health" _x _y (* (/ (Math|Conversions|ToFloat(Integer) _health) 1e+02) 128.0) 16.0 0.0 0.5 (/ (Math|Conversions|ToFloat(Integer) _health) 1e+02) 0.5 "(R=1.000000,G=1.000000,B=1.000000,A=1.000000)" "BLEND_Translucent" InScale true)
  (Canvas|DrawTexture "/Game/Textures/Health.Health" _x _y 128.0 16.0 0.0 0.0 1.0 0.5 "(R=1.000000,G=1.000000,B=1.000000,A=1.000000)" "BLEND_Translucent" InScale true))

(fn GetHealth
  (return 0))

(fn GetScore
  (return 0))