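; Player ship Blueprint for a shooter, steered by mouse along a clamped Y axis.
; Left click spawns a bullet above the ship, or opens the Title level once the ship is hidden, which serves as the game-over state.
; Overlaps spawn explosions, while damage lowers Health until the ship explodes, hides and disables collision.
; Getters expose Health and a Score that is always zero.
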(event Collision|EventActorBeginOverlap
  (params (OtherActor :type Actor%20Object%20Reference))
  ;[1 1 1] 弾があたった時
  (Game|SpawnActorfromClass "/Game/StarterContent/Blueprints/Blueprint_Effect_Explosion.Blueprint_Effect_Explosion_C" (Math|Conversions|ToTransform(Vector) (Transformation|GetActorLocation)) "Undefined" 0 0))

(event Game|Damage|EventAnyDamage
  (params (Damage :type Float%20%28single-precision%29) (DamageType :type Damage%20Type%20Object%20Reference) (InstigatedBy :type Controller%20Object%20Reference) (DamageCauser :type Actor%20Object%20Reference))
  ;[1 1 1] ダメージ追加
  (bind _output_get (Variables|Default|SetHealth (- (Variables|Default|GetHealth) (Math|Float|Floor Damage))))
  ;[1 1 1] 自機破壊
  (if (<= _output_get 0)
    (Game|SpawnActorfromClass "/Game/StarterContent/Blueprints/Blueprint_Effect_Explosion.Blueprint_Effect_Explosion_C" (Math|Conversions|ToTransform(Vector) (Transformation|GetActorLocation)) "Undefined" 0 0)
    (Rendering|SetActorHiddenInGame true)
    (Collision|SetActorEnableCollision false)))

(event Input|MouseEvents|MouseX
  (params (AxisValue :type Float%20%28single-precision%29))
  (bind _returnvalue (Transformation|GetActorLocation))
  (bind _returnvalue_2 (* "0,10.000000,0.000000" AxisValue))
  (bind _returnvalue_3 (+ _returnvalue _returnvalue_2))
  (bind (_x _y _z) (Math|Vector|BreakVector _returnvalue_3))
  ;[1 1 1] 移動
  (Transformation|SetActorLocation (Math|Vector|MakeVector _x (Math|Float|Min(Float) (Math|Float|Max(Float) _y -4e+02) 4e+02) _z) false false))

(event Input|MouseEvents|LeftMouseButton
  (params (Key :type Key%20Structure :default "AnyKey"))
  (:Pressed
    ;[1 1 1] 弾の発射/タイトルに戻る
    (if (Variables|Rendering|GetbHidden) ; 自機が消えている場合はゲームオーバーとみなす
      (Game|OpenLevel(byName) "Title") ; クリックしてタイトルへ戻る
      (else
        (Game|SpawnActorfromClass "/Game/Blueprints/PlayerBulletBlueprint.PlayerBulletBlueprint_C" (Math|Conversions|ToTransform(Vector) (+ (Transformation|GetActorLocation) "0, 0,50.000000")) "Undefined" 0 0) ; 弾の発射
      ))))

(fn ConstructionScript)

(fn GetHealth
  (return (Variables|Default|GetHealth)))

(fn GetScore
  (return 0))